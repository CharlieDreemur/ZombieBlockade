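; Base enemy character that chases the player, makes melee attacks and dies when its health runs out.
; Tick reissues an AI move to the player, falling back to the nearest building if that fails.
; On arrival, a CanAttack-gated montage plays while delayed, range-checked damage hits only the player, even at buildings.
; Incoming damage reduces Health; lethal hits play a death animation, then destroy the actor after a delay.
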(event `self.ReceiveBeginPlay`)

(event `self.ReceiveTick`
  (params (DeltaSeconds :type "Float (single-precision)"))
  (if (not (`self.IsDead`))
    (`self.FollowPlayer`)))

(event `self.ReceiveAnyDamage`
  (params (Damage :type "Float (single-precision)") (DamageType :type "DamageType Object Reference") (InstigatedBy :type "Controller Object Reference") (DamageCauser :type "Actor Object Reference"))
  (`self.Receive Damage` Damage)
  (`KismetSystemLibrary.PrintString` (`KismetStringLibrary.Conv_DoubleToString` (`self.Health`))))

(event `Death`
  (set `self.IsDead` true)
  (`SkeletalMeshComponent.PlayAnimation` (`self.Mesh`) "/Game/Fantasy_RPG_Game/Animations/Zombie/Root_Motion/Death_RM_Anim.Death_RM_Anim" false)
  (`MovementComponent.StopMovementImmediately` (`self.CharacterMovement`))
  (`KismetSystemLibrary.Delay` 2.5)
  (`self.K2_DestroyActor`))

(event `FollowPlayer`
  (bind (_returnvalue_x _returnvalue_y) (`KismetMathLibrary.BreakVector` (`self.K2_GetActorLocation`)))
  (if (not (`self.IsDead`))
    (`|AIMoveTo` self (0.0 0.0 0.0) (`GameplayStatics.GetPlayerPawn` 0)
      (:`OnSuccess`
        _)
      (:`OnFail`
        (set `self.FirstTime` true)
        (bind _returnvalue (`GridManager.Instance`))
        (`|AIMoveTo` null (0.0 0.0 0.0) (`GridManager.FindNearestBuilding` _returnvalue (`KismetMathLibrary.MakeVector2D` _returnvalue_x _returnvalue_y))
          (:`OnSuccess`
            _))))
    (if (`self.FirstTime`)
      (set `self.FirstTime` false)
      (else
        (`KismetSystemLibrary.Delay` 1.2)))
    (if (`self.CanAttack`)
      (set `self.CanAttack` false)
      (`|ExecutionSequence`
        (:`then_0`
          (`KismetSystemLibrary.Delay` (* (`self.AttackAnimationPlayRate`) 0.6))
          (if (<= (`self.GetDistanceTo` self (`GameplayStatics.GetPlayerCharacter` 0)) 120.0)
            (`GameplayStatics.ApplyDamage` (`GameplayStatics.GetPlayerCharacter` 0) 10.0)))
        (:`then_1`
          (bind _returnvalue_2 (`self.PlayAnimMontage` "/Game/Animation/Enemy/Attack.Attack" (`self.AttackAnimationPlayRate`)))
          (`KismetSystemLibrary.Delay` (+ _returnvalue_2 (`self.AttackDelayedTime`)))
          (set `self.CanAttack` true))))))

(fn `Perform Attack`)

(fn `Receive Damage`
  (params (DamageAmount :type "Float (double-precision)"))
  (bind _returnvalue (- (`self.Health`) DamageAmount))
  (if (<= _returnvalue 0.0)
    (if (not (`self.IsDead`))
      (`self.Death`))
    (else
      (set `self.Health` _returnvalue))))

(fn `UserConstructionScript`)