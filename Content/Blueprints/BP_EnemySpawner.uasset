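; Enemy spawner that spawns base enemies and fast zombies in waves, triggered by the player controller's respawn event.
; Counts come from WaveTable for waves below 6, then each grows by one per call.
; Spawns use random TargetPoints, capped by their number, and CurrWave increments per fast zombie spawned, not per wave.
; Tick also steps XValues and YValues around a square via a four-state cycle, unused by spawning.
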(event `self.ReceiveTick`
  (params (DeltaSeconds :type "Float (single-precision)"))
  (`self.generatevalues`))

(event `self.ReceiveBeginPlay`
  (bind _asbp_top_down_player_controller (cast `/Game/TopDown/Blueprints/BP_TopDownPlayerController` (`GameplayStatics.GetPlayerController` 0)))
  (add `/Game/TopDown/Blueprints/BP_TopDownPlayerController.RespawnEnemy` _asbp_top_down_player_controller (delegate `SpawnEnemy`)))

(event `SpawnEnemy`
  (bind _currwave (`self.currWave`))
  (if (>= _currwave 6)
    (set `self.Enemy A` (+ (`self.Enemy A`) 1))
    (set `self.Enemy B` (+ (`self.Enemy B`) 1))
    (else
      (bind _outrownames (`DataTableFunctionLibrary.GetDataTableRowNames` "/Game/Blueprints/WaveTable.WaveTable"))
      (bind _returnvalue (`|GetDataTableRow` "/Game/Blueprints/WaveTable.WaveTable" (`|GetArrayItem` _outrownames _currwave))
        (:`then`
          (bind (_wavenum _enemya _enemyb) (break `/Game/Blueprints/Wave` _returnvalue))
          (set `self.Enemy A` _enemya)
          (set `self.Enemy B` _enemyb)))))
  (bind _outactors (`GameplayStatics.GetAllActorsOfClass` "/Script/Engine.TargetPoint"))
  (for (_ _array_index) _outactors
    (if (>= _array_index (`self.Enemy A`))
      (break)
      (else
        (`|SpawnActorFromClass` "/Game/Blueprints/BP_EnemyBase.BP_EnemyBase_C" (`self.GetTransform` (`KismetArrayLibrary.Array_Random` _outactors)) "Undefined" "MultiplyWithRoot" null null))))
  (bind _outactors_2 (`GameplayStatics.GetAllActorsOfClass` "/Script/Engine.TargetPoint"))
  (for (_ _array_index_2) _outactors_2
    (if (>= _array_index_2 (`self.Enemy B`))
      (break)
      (else
        (`|SpawnActorFromClass` "/Game/Blueprints/BP_FastNormalZombie.BP_FastNormalZombie_C" (`self.GetTransform` (`KismetArrayLibrary.Array_Random` _outactors_2)) "Undefined" "MultiplyWithRoot" null null)
        (bind _result (`/Engine/EditorBlueprintResources/StandardMacros.IncrementInt` (`self.currWave`))
          (:`  `
            (set `self.currWave` _result)))))))

(fn `generatevalues`
  (bind _y_values (`self.Y_values`))
  (bind _y_values_2 (`self.Y_values`))
  (bind _x_values (`self.X_values`))
  (bind _x_values_2 (`self.X_values`))
  (switch `int` (`self.State`)
    (:`0`
      (if (<= _x_values 2500.0)
        (set `self.X_values` (+ (`self.Increment`) _x_values))
        (else
          (set `self.State` 1))))
    (:`1`
      (if (<= _y_values_2 2500.0)
        (set `self.Y_values` (+ (`self.Increment`) _y_values_2))
        (else
          (set `self.State` 2))))
    (:`2`
      (if (>= _x_values_2 500.0)
        (set `self.X_values` (- _x_values_2 (`self.Increment`)))
        (else
          (set `self.State` 3))))
    (:`3`
      (if (>= _y_values 500.0)
        (set `self.Y_values` (- _y_values (`self.Increment`)))
        (else
          (set `self.State` 0))))))

(fn `UserConstructionScript`)