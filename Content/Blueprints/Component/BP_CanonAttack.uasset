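; Actor component that gives a Building an automatic cannon attack against nearby enemies.
; A looping timer picks the nearest living BP_EnemyBase overlapping the owner's SphereComponent, keeping the previous target if none is found.
; While that target is valid, it spawns a Weapon_canon at the "ShootPosition"-tagged component, yawed toward the enemy with a fixed upward pitch.
; The projectile homes on the target, with damage scaled by the building's level.
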(event `self.ReceiveEndPlay`
  (params (EndPlayReason :type "EEndPlayReason Enum" :default "Destroyed"))
  (`KismetSystemLibrary.K2_ClearAndInvalidateTimerHandle` (stale `self.ReceiveBeginPlay` _returnvalue)))

(event `self.ReceiveTick`
  (params (DeltaSeconds :type "Float (single-precision)")))

(event `self.ReceiveBeginPlay`
  (set `self.SphereComponent` (`Actor.GetComponentByClass` (`self.GetOwner`) "/Script/Engine.SphereComponent"))
  (bind _returnvalue (`KismetSystemLibrary.K2_SetTimerDelegate` (delegate `DetectEnemy`) (`self.AttackInterval`) true)))

(event `AttackEnemy`
  (bind _targetenemy (`self.TargetEnemy`))
  (bind _returnvalue (`SceneComponent.K2_GetComponentLocation` (`|GetArrayItem` (`Actor.GetComponentsByTag` (`self.GetOwner`) "/Script/Engine.SceneComponent" "ShootPosition"))))
  (bind (_returnvalue_roll _returnvalue_pitch _returnvalue_yaw) (`KismetMathLibrary.BreakRotator` (`KismetMathLibrary.FindLookAtRotation` _returnvalue (`Actor.K2_GetActorLocation` _targetenemy))))
  (`/Engine/EditorBlueprintResources/StandardMacros.IsValid` _targetenemy
    (:`Is Valid`
      (bind _returnvalue_2 (`|SpawnActorFromClass` "/Game/Blueprints/Weapon_canon.Weapon_canon_C" (`KismetMathLibrary.MakeTransform` _returnvalue (`KismetMathLibrary.MakeRotator` _returnvalue_roll 45.0 _returnvalue_yaw)) "Undefined" "MultiplyWithRoot" null null))
      (`/Engine/EditorBlueprintResources/StandardMacros.IsValid` _returnvalue_2
        (:`Is Valid`
          (bind _asbuilding (cast `Building` (`self.GetOwner`)))
          (set `/Game/Blueprints/Weapon_canon.Damage` (* (`Building.GetCurrentLevel` _asbuilding) (`self.AttackDamage`)) _returnvalue_2)
          (`/Game/Blueprints/Weapon_canon.SetHoming` _returnvalue_2 _targetenemy))))))

(event `DetectEnemy`
  (set `self.MinDistance` 999999999.0)
  (for _array_element (`PrimitiveComponent.GetOverlappingActors` (`self.SphereComponent`) "/Game/Blueprints/Zombies/BP_EnemyBase.BP_EnemyBase_C")
    (bind _asbp_enemy_base (cast `/Game/Blueprints/Zombies/BP_EnemyBase` _array_element))
    (if (not (`/Game/Blueprints/Zombies/BP_EnemyBase.IsDead` _asbp_enemy_base))
      (bind _returnvalue (`KismetMathLibrary.VSizeSquared` (- (`Actor.K2_GetActorLocation` _array_element) (`Actor.K2_GetActorLocation` (`self.GetOwner`)))))
      (if (< _returnvalue (`self.MinDistance`))
        (set `self.MinDistance` _returnvalue)
        (set `self.TargetEnemy` _array_element))))
  (`self.AttackEnemy`))