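; BP_EconomyComponent is an actor component that generates passive income for the Building that owns it.
; Each Tick adds delta time to a running timer and divides it by the generation interval, keeping the remainder so no time is lost.
; Completed intervals are multiplied by the generate amount and the building's current level, then paid through AddMoney on a shared instance.
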(event `self.ReceiveTick`
  (params (DeltaSeconds :type "Float (single-precision)"))
  (bind (_remainder _returnvalue) (`KismetMathLibrary.FMod` (+ DeltaSeconds (`self.CurrentTime`)) (`self.GenerateInterval`)))
  (bind _asbuilding (cast `Building` (`self.GetOwner`)))
  (set `self.CurrentTime` _remainder)
  (if (`KismetMathLibrary.Conv_IntToBool` _returnvalue)
    (bind _returnvalue_2 (`Economy.Instance`))
    (`Economy.AddMoney` _returnvalue_2 (* _returnvalue (`self.GenerateAmount`) (`Building.GetCurrentLevel` _asbuilding)))))