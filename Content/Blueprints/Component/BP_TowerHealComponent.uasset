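; Actor component that makes a tower building periodically heal the most damaged building in its range.
; A looping timer scans Buildings overlapping the owner's SphereComponent for the lowest health percentage below full.
; It heals that target by HealAmount times the tower's level, spawning light and beam effects at the shoot point and target.
; The target is never cleared, so the last one keeps being healed when none are damaged.
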(event `self.ReceiveEndPlay`
  (params (EndPlayReason :type "EEndPlayReason Enum" :default "Destroyed"))
  (`KismetSystemLibrary.K2_ClearAndInvalidateTimerHandle` (stale `self.ReceiveBeginPlay` _returnvalue)))

(event `self.ReceiveTick`
  (params (DeltaSeconds :type "Float (single-precision)")))

(event `self.ReceiveBeginPlay`
  (set `self.SphereComponent` (`Actor.GetComponentByClass` (`self.GetOwner`) "/Script/Engine.SphereComponent"))
  (bind _returnvalue (`KismetSystemLibrary.K2_SetTimerDelegate` (delegate `DetectMinHealthBuilding`) (`self.AttackInterval`) true)))

(event `HealBuilding`
  (bind _returnvalue (`self.GetOwner`))
  (bind _targetbuilding (`self.TargetBuilding`))
  (bind _returnvalue_2 (`Actor.K2_GetActorLocation` _targetbuilding))
  (`/Engine/EditorBlueprintResources/StandardMacros.IsValid` _targetbuilding
    (:`Is Valid`
      (bind _asbuilding (cast `Building` _returnvalue))
      (`Building.AddHealth` (`self.TargetBuilding`) (* (`Building.GetCurrentLevel` _asbuilding) (`self.HealAmount`)))
      (`|SpawnActorFromClass` "/Game/Blueprints/VFX/BP_HealLight.BP_HealLight_C" (`KismetMathLibrary.MakeTransform` (`SceneComponent.K2_GetComponentLocation` (`|GetArrayItem` (`Actor.GetComponentsByTag` _returnvalue "/Script/Engine.SceneComponent" "ShootPosition")))) "Undefined" "MultiplyWithRoot" null null)
      (`|SpawnActorFromClass` "/Game/Blueprints/VFX/BP_VFX_Healbeam.BP_VFX_Healbeam_C" (`KismetMathLibrary.MakeTransform` _returnvalue_2) "Undefined" "MultiplyWithRoot" null null)
      (`|SpawnActorFromClass` "/Game/Blueprints/VFX/BP_HealLight.BP_HealLight_C" (`KismetMathLibrary.MakeTransform` (+ _returnvalue_2 (50.0 50.0 100.0))) "Undefined" "MultiplyWithRoot" null null))))

(event `DetectMinHealthBuilding`
  (set `self.MinHealthPercentage` 1.0)
  (for _array_element (`PrimitiveComponent.GetOverlappingActors` (`self.SphereComponent`) "/Script/ZombieBlockade.Building")
    (bind _asbuilding (cast `Building` _array_element))
    (bind _returnvalue (`Building.GetHealthPercentage` _asbuilding))
    (if (< _returnvalue (`self.MinHealthPercentage`))
      (set `self.MinHealthPercentage` _returnvalue)
      (set `self.TargetBuilding` _asbuilding)))
  (`self.HealBuilding`))