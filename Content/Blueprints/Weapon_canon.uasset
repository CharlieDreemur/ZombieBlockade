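; Cannonball projectile weapon that can home in on a target and explodes when it overlaps an enemy.
; SetHoming stores the target and points the ProjectileMovement homing at that enemy's mesh component.
; Any overlap plays the shooting sound, but only a BP_EnemyBase spawns a BP_Explosion at the enemy's location, passing Damage on, and destroys the projectile.
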(event `self.ReceiveActorBeginOverlap`
  (params (OtherActor :type "Actor Object Reference"))
  (`GameplayStatics.PlaySound2D` "/Game/Music-Sound/CanonBall_Shooting.CanonBall_Shooting" 1.0 1.0 0.0 null null)
  (bind _asbp_enemy_base (cast `/Game/Blueprints/Zombies/BP_EnemyBase` OtherActor))
  (`|SpawnActorFromClass` "/Game/Blueprints/VFX/BP_Explosion.BP_Explosion_C" (`KismetMathLibrary.MakeTransform` (`self.K2_GetActorLocation` _asbp_enemy_base)) "Undefined" "MultiplyWithRoot" null (`self.Damage`) null)
  (`self.K2_DestroyActor`))

(event `SetHoming`
  (params (Enemy :type "Actor Object Reference"))
  (bind _projectilemovement (`self.ProjectileMovement`))
  (set `self.HomingTarget` Enemy)
  (set `ProjectileMovementComponent.bIsHomingProjectile` true _projectilemovement)
  (set `ProjectileMovementComponent.HomingTargetComponent` (`self.GetComponentByClass` Enemy "/Script/Engine.MeshComponent") _projectilemovement))

(fn `UserConstructionScript`)