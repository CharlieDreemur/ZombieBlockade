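; Base zombie enemy character that hunts the player or nearby buildings, with stats supplied through Init.
; A one-second timer retargets to the player if the Instance reports them reachable, otherwise to the nearest building, then moves via AIMoveTo.
; Arrival sets attack flags, and the animation-finish event applies damage within range or drops out of attacking.
; Incoming damage reduces health until death, which adds score and destroys the actor after a delay.
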(event `self.ReceiveBeginPlay`
  (if (not (`self.IsDead`))
    (`self.FindTarget`)
    (`KismetSystemLibrary.K2_SetTimerDelegate` (delegate `FindTarget`) 1.0 true)))

(event `self.ReceiveTick`
  (params (DeltaSeconds :type "Float (single-precision)")))

(event `self.ReceiveAnyDamage`
  (params (Damage :type "Float (single-precision)") (DamageType :type "DamageType Object Reference") (InstigatedBy :type "Controller Object Reference") (DamageCauser :type "Actor Object Reference"))
  (`self.Receive Damage` Damage)
  (`KismetSystemLibrary.PrintString` (`KismetStringLibrary.Conv_IntToString` (`self.Health`))))

(event `Death`
  (set `self.IsDead` true)
  (`MovementComponent.StopMovementImmediately` (`self.CharacterMovement`))
  (`Economy.AddScore` (`Economy.Instance`) 1)
  (`KismetSystemLibrary.Delay` 2.5)
  (`self.K2_DestroyActor`))

(event `FindTarget`
  (bind (_returnvalue_x _returnvalue_y) (`KismetMathLibrary.BreakVector` (`self.K2_GetActorLocation`)))
  (bind (_returnvalue_x_2 _returnvalue_y_2) (`KismetMathLibrary.BreakVector` (`self.K2_GetActorLocation`)))
  (bind (_returnvalue_x_3 _returnvalue_y_3) (`KismetMathLibrary.BreakVector` (`self.K2_GetActorLocation` (`GameplayStatics.GetPlayerPawn` 0))))
  (if (not (or false (`self.IsDead`)))
    (if (`GridManager.CanReachLocation` (`GridManager.Instance`) (`KismetMathLibrary.MakeVector2D` _returnvalue_x_2 _returnvalue_y_2) (`KismetMathLibrary.MakeVector2D` _returnvalue_x_3 _returnvalue_y_3))
      (`self.SetNewTarget` (`GameplayStatics.GetPlayerPawn` 0))
      (else
        (`self.SetNewTarget` (`GridManager.FindNearestBuilding` (`GridManager.Instance`) (`KismetMathLibrary.MakeVector2D` _returnvalue_x _returnvalue_y)))))
    (if (not (`self.IsAttack`))
      (`|AIMoveTo` self (0.0 0.0 0.0) (`self.AttackTarget`)
        (:`OnSuccess`
          (if (`self.FirstTime`)
            (set `self.FirstTime` false))
          (if (`self.CanAttack`)
            (set `self.IsAttack` true)
            (set `self.CanAttack` false)))))))

(event `OnFinishAttackAnimation`
  (set `self.CanAttack` true)
  (if (<= (`self.GetDistanceTo` self (`self.AttackTarget`)) 120.0)
    (`GameplayStatics.ApplyDamage` (`self.AttackTarget`) (`KismetMathLibrary.Conv_IntToDouble` (`self.BasicDamage`)))
    (else
      (set `self.IsAttack` false))))

(fn `Init`
  (params (Health :type Integer) (BasicDamage :type Integer) (AttackAnimationPlayRate :type "Float (double-precision)") (WalkAnimationPlayRate :type "Float (double-precision)"))
  (set `self.Health` Health)
  (set `self.BasicDamage` BasicDamage)
  (set `self.AttackAnimationPlayRate` AttackAnimationPlayRate)
  (set `self.WalkAnimationPlayRate` WalkAnimationPlayRate))

(fn `Perform Attack`)

(fn `Receive Damage`
  (params (DamageAmount :type "Float (double-precision)"))
  (bind _returnvalue (- (`self.Health`) DamageAmount))
  (if (<= _returnvalue 0.0)
    (if (not (`self.IsDead`))
      (`self.Death`))
    (else
      (set `self.Health` (`KismetMathLibrary.FTrunc` _returnvalue)))))

(fn `SetNewTarget`
  (params (Target :type "Actor Object Reference"))
  (if (not (== Target (`self.AttackTarget`)))
    (set `self.AttackTarget` Target)
    (`MovementComponent.StopMovementImmediately` (`self.CharacterMovement`))))

(fn `UserConstructionScript`)